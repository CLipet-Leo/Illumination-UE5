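; BP_Cards is an interactable card prop that turns a quarter turn per interaction, cycling its current face through Valet, King, Queen and Princess.
; Interact ignores input while animating, advances the value, and computes a target 90 degrees from the Cards component's current rotation.
; A shared timeline lerps to that rotation along the shortest path, then releases the lock.
; Interaction getters return fixed values, keeping it always activated with zero hold time.
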(event EventBeginPlay)

(event Collision|EventActorBeginOverlap
  (params (OtherActor :type Actor%20Object%20Reference)))

(event EventTick
  (params (DeltaSeconds :type Float%20%28single-precision%29)))

(event EventInteract
  (params (InteractActorRef :type Actor%20Object%20Reference))
  (if (not (Variables|Default|GetbInAnimation))
    (Variables|Default|SetbInAnimation true)
    (bind _output_get (Variables|Default|SetActualRotation (Variables|/Script/Engine.SceneComponent|GetRelativeRotation (Variables|Default|GetCards))))
    (Variables|Default|SetTargetRotation (Math|Rotator|CombineRotators _output_get "0.000000,90.000000,0.000000"))
    (switch Utilities|FlowControl|Switch|SwitchonEnum_Cards (Variables|Default|GetCurrentValue)
      (:NewEnumerator0
        (Variables|Default|SetCurrentValue "NewEnumerator1")
        (bind _alpha (Timeline|TL_Rotation PlayFromStart)
          (:Update
            (Transformation|SetRelativeRotation (Variables|Default|GetCards) (Math|Rotator|Lerp(Rotator) (Variables|Default|GetActualRotation) (Variables|Default|GetTargetRotation) _alpha true) false false))
          (:Finished
            (Variables|Default|SetbInAnimation false))))
      (:NewEnumerator1
        (Variables|Default|SetCurrentValue "NewEnumerator2")
        (Timeline|TL_Rotation PlayFromStart))
      (:NewEnumerator2
        (Variables|Default|SetCurrentValue "NewEnumerator3")
        (Timeline|TL_Rotation PlayFromStart))
      (:NewEnumerator3
        (Variables|Default|SetCurrentValue "NewEnumerator0")
        (Timeline|TL_Rotation PlayFromStart)))))

(fn ConstructionScript)

(fn GetHoldDuration
  (return 0.0))

(fn GetInteractionType
  (return "NewEnumerator0"))

(fn GetIsActivated
  (return true))

(fn GetWidgetOffsetComp
  (return 0))