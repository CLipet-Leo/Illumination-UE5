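; BP_IronBars is a set of iron bars that slides down to open and back up to close.
; BeginPlay derives the open position from the mesh's bounds height plus a small margin, and starts the bars lowered if IsOpen is set.
; ToggleBars flips IsOpen and plays or reverses a timeline that lerps the mesh's relative location between closed and open positions.
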(event Custom|ToggleBars
  (bind _output_get (Variables|Default|SetbIsOpen (not (Variables|Default|GetbIsOpen))))
  (if _output_get
    (bind _alpha (Timeline|TL_AnimBarreaux Play)
      (:Update
        (Transformation|SetRelativeLocation (Variables|Default|GetMesh) (Math|Vector|Lerp(Vector) (Variables|Default|GetBasePosition) (Variables|Default|GetOpenPosition) _alpha) false false)))
    (else
      (Timeline|TL_AnimBarreaux Reverse))))

(event EventBeginPlay
  (bind _mesh (Variables|Default|GetMesh))
  (Variables|Default|SetBasePosition (Variables|/Script/Engine.SceneComponent|GetRelativeLocation _mesh))
  (Variables|Default|SetOpenPosition (Math|Vector|MakeVector (.x (Variables|Default|GetBasePosition)) (.y (Variables|Default|GetBasePosition)) (- (- (.z (Variables|Default|GetBasePosition)) (* (.Z (Math|Vector|BreakVector (.BoxExtent (Collision|GetComponentBounds _mesh)))) 2.0)) 1e+01)))
  (if (Variables|Default|GetbIsOpen)
    (Transformation|SetRelativeLocation (Variables|Default|GetMesh) (Variables|Default|GetOpenPosition) false false)
    (Components|Timeline|SetPlaybackPosition (Variables|Default|GetTL_AnimBarreaux) 1.0 false false)))

(fn ConstructionScript)