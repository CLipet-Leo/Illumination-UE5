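; BP_Lever is an interactable lever that toggles on each Interact and registers or unregisters itself with a target door's lever array.
; A timeline plays or reverses to lerp the handle mesh's pitch between its BeginPlay rotation and an activated offset.
; Interaction getters return a zero hold duration, a fixed interaction type and no widget offset component.
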(event EventBeginPlay
  (Variables|Default|SetBaseRotation (Variables|/Script/Engine.SceneComponent|GetRelativeRotation (Variables|Default|GetCube1))))

(event EventInteract
  (params (InteractActorRef :type Actor%20Object%20Reference))
  (bind _baserotation (Variables|Default|GetBaseRotation))
  (bind _pitch (Math|Rotator|BreakRotator _baserotation))
  (if (Variables|Default|GetbActivated)
    (Development|PrintString "Flop B")
    (Variables|Default|SetbActivated false)
    (Default|RemoveLeverfromArray (Variables|Default|GetTargetDoor) self)
    (bind _levertrack (Timeline|Timeline Reverse)
      (:Update
        (Transformation|SetRelativeRotation (Variables|Default|GetCube1) (Math|Rotator|MakeRotator 0.0 (Math|Float|Lerp _pitch (+ _pitch (.Pitch (Math|Rotator|BreakRotator (Variables|Default|GetActivatedOffset)))) _levertrack) 0.0) false false)))
    (else
      (Development|PrintString "Flip A")
      (Variables|Default|SetbActivated true)
      (Default|AddLevertoArray (Variables|Default|GetTargetDoor) self)
      (Timeline|Timeline Play))))

(fn ConstructionScript)

(fn GetHoldDuration
  (return 0.0))

(fn GetInteractionType
  (return "NewEnumerator0"))

(fn GetWidgetOffsetComp
  (return 0))