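; Puzzle manager for a memory game where the player repeats a random sequence of lights to open a door.
; It fills an index map with random light indices, and the SequencePlayer's activation event replays them through a self-rescheduling timer.
; Light interactions are checked in order: completion opens DoorRef, while a mistake resets the lights and rolls a new sequence.
; Only the easy difficulty is implemented.
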(event Custom|PlaySequence
  (Utilities|FlowControl|Delay 1.0)
  (Development|PrintString "Playing Sequence")
  (Variables|Logic|SetplayingIndex 0)
  (CallFunction|PlaySequenceStep)
  (if (< (Variables|Logic|GetplayingIndex) (Utilities|Map|Length (Variables|Logic|GetIndexMap)))
    (Utilities|Time|SetTimerbyEvent (delegate Custom|CustomEvent) (+ (Variables|Logic|GetTimeToSwitch) (Variables|Logic|GetDelayToSwitch)))
    (else
      (Variables|Logic|SetplayingIndex 0)
      (Development|PrintString "Finished Sequence"))))

(event Custom|InitSequence
  (params (isEasy :type Boolean))
  (if isEasy
    (CallFunction|InitializeSequence 1.4 4)))

(event Custom|LightInteraction
  (params (CallingActorRef :type BP%20Light%20Lever%20Object%20Reference))
  (if (== (.Value (Utilities|Map|GetKeyValueByIndex (Variables|Logic|GetIndexMap) (Variables|Logic|GetplayingIndex))) (Utilities|Array|FindItem (Variables|Manager|GetLightArray) CallingActorRef))
    (Variables|Logic|SetplayingIndex (+ (Variables|Logic|GetplayingIndex) 1))
    (if (== (Variables|Logic|GetplayingIndex) (Utilities|Map|Length (Variables|Logic|GetIndexMap)))
      (CallFunction|WinFunc))
    (else
      (CallFunction|ResetSequence))))

(event Custom|CustomEvent
  (CallFunction|PlaySequenceStep)
  (if (< (Variables|Logic|GetplayingIndex) (Utilities|Map|Length (Variables|Logic|GetIndexMap)))
    (Utilities|Time|SetTimerbyEvent (delegate Custom|CustomEvent) (+ (Variables|Logic|GetTimeToSwitch) (Variables|Logic|GetDelayToSwitch)))
    (else
      (Variables|Logic|SetplayingIndex 0)
      (Development|PrintString "Finished Sequence"))))

(event EventBeginPlay
  (bind _sequenceplayer (Variables|Manager|GetSequencePlayer))
  (if (Utilities|Array|IsEmpty (Variables|Manager|GetLightArray))
    (CallFunction|NewError " LigthArray is empty")
    (elif (not (Utilities|IsValid (Variables|Manager|GetDoorRef)))
      (CallFunction|NewError " DoorRef is empty")
      (else
        (Variables|Logic|SetLength (Utilities|Array|Length (Variables|Manager|GetLightArray)))
        (CallFunction|InitSequence (Variables|Logic|GetisEasy))
        (Utilities|IsValid _sequenceplayer
          (:Is%20Valid
            (EventDispatchers|BindEventtoSendActivation _sequenceplayer (delegate Custom|PlaySequence))
            (for _array_element (Variables|Manager|GetLightArray)
              (EventDispatchers|BindEventtoCallInteraction _array_element (EventDispatchers|CreateEvent :!event Custom|LightInteraction)))))))))

(fn ConstructionScript)

(fn InitializeSequence
  (params (TimeToSwitch :type Float%20%28double-precision%29) (NumberOfIteraction :type Integer))
  (Variables|Logic|SetTimeToSwitch TimeToSwitch)
  (if (Utilities|Map|IsEmpty (Variables|Logic|GetIndexMap))
    _
    (else
      (Utilities|Map|Clear (Variables|Logic|GetIndexMap))))
  (for _index (range 0 (- NumberOfIteraction 1))
    (Utilities|Map|Add (Variables|Logic|GetIndexMap) _index (.OutIndex (Utilities|Array|Random (Variables|Manager|GetLightArray)))))
  (bind (_keypin _valuepin) (Utilities|Map|ForEachLoop(Map) (Variables|Logic|GetIndexMap))
    (:then
      (Development|PrintString (Utilities|String|Append "Key : " (Utilities|String|ToString(Integer) _keypin) " / Value : " (Utilities|String|ToString(Integer) _valuepin)) true true "(R=1.000000,G=0.000000,B=0.864332,A=1.000000)" 5.0))))

(fn PlaySequenceStep
  (Development|PrintString (Utilities|String|Append "Step : " (Utilities|String|ToString(Integer) (Variables|Logic|GetplayingIndex))))
  (Class|BPILightLever|TurnLightfor(Message) (Utilities|Array|Get(acopy) (Variables|Manager|GetLightArray) (.Value (Utilities|Map|GetKeyValueByIndex (Variables|Logic|GetIndexMap) (Variables|Logic|GetplayingIndex)))) 0.0 (Variables|Logic|GetTimeToSwitch))
  (Variables|Logic|SetplayingIndex (+ (Variables|Logic|GetplayingIndex) 1)))

(fn ResetSequence
  (Class|BPILever|SetState(Message) (Variables|Manager|GetSequencePlayer) false)
  (for _array_element (Variables|Manager|GetLightArray)
    (Class|BPILightLever|Reset(Message) _array_element))
  (Variables|Logic|SetplayingIndex 0)
  (CallFunction|InitSequence true))

(fn WinFunc
  (Development|PrintString "YOU WIN !!!!!!" true true "(R=0.000000,G=1.000000,B=0.009109,A=1.000000)" 5.0)
  (Default|OpenDoor (Variables|Manager|GetDoorRef)))

(fn NewError
  (params (Message :type String))
  (Utilities|Debugging|RaiseScriptError (Utilities|String|Append (Utilities|GetDisplayName self) Message)))