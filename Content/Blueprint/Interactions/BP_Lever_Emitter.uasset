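; Interactable lever emitter that sends an activation signal when first used, then locks out further interaction.
; A FlipFlop alternately plays and reverses a timeline that lerps the cube's pitch between its starting angle and an offset.
; SetState changes the active state without sending activation, re-enabling interaction when deactivated.
; GetIsActive always returns false, independent of the Activated flag.
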(event EventBeginPlay
  (Variables|Default|SetBaseRotation (Variables|/Script/Engine.SceneComponent|GetRelativeRotation (Variables|Default|GetCube1))))

(event EventInteract
  (params (InteractActorRef :type Actor%20Object%20Reference))
  (if (not (Variables|Default|GetbActivated))
    (Default|CallSendActivation)
    (CallFunction|ToggleState)
    (Variables|Default|SetCan%20Interact false)))

(event EventSetState
  (params (newIsActive :type Boolean))
  (bind _baserotation (Variables|Default|GetBaseRotation))
  (bind _pitch (Math|Rotator|BreakRotator _baserotation))
  (if (!= newIsActive (Variables|Default|GetbActivated))
    (Variables|Default|SetbActivated newIsActive)
    (Variables|Default|SetCan%20Interact (not newIsActive))
    (Utilities|FlowControl|FlipFlop
      (:A
        (bind _levertrack (Timeline|Timeline Play)
          (:Update
            (Transformation|SetRelativeRotation (Variables|Default|GetCube1) (Math|Rotator|MakeRotator 0.0 (Math|Float|Lerp _pitch (+ _pitch (.Pitch (Math|Rotator|BreakRotator (Variables|Default|GetActivatedOffset)))) _levertrack) 0.0) false false))))
      (:B
        (Timeline|Timeline Reverse)))))

(event EventToggleState
  (bind _baserotation (Variables|Default|GetBaseRotation))
  (bind _pitch (Math|Rotator|BreakRotator _baserotation))
  (Variables|Default|SetbActivated (not (Variables|Default|GetbActivated)))
  (Utilities|FlowControl|FlipFlop
    (:A
      (bind _levertrack (Timeline|Timeline Play)
        (:Update
          (Transformation|SetRelativeRotation (Variables|Default|GetCube1) (Math|Rotator|MakeRotator 0.0 (Math|Float|Lerp _pitch (+ _pitch (.Pitch (Math|Rotator|BreakRotator (Variables|Default|GetActivatedOffset)))) _levertrack) 0.0) false false))))
    (:B
      (Timeline|Timeline Reverse))))

(fn ConstructionScript)

(fn GetCanInteract
  (return (Variables|Default|GetCan%20Interact)))

(fn GetHoldDuration
  (return 0.0))

(fn GetInteractionType
  (return "NewEnumerator0"))

(fn GetIsActive
  (return false))

(fn GetWidgetOffsetComp
  (return 0))