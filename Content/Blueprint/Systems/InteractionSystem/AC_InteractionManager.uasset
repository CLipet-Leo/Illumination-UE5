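; Character component that finds nearby BPI_Interactable actors and handles interacting with the closest one.
; A looping timer runs a sphere overlap, filters by interactability and line trace, then selects the nearest actor.
; The InteractableRef RepNotify rebuilds a screen-space prompt widget at that actor.
; Press interacts immediately, while Hold binds a dispatcher fed by input elapsed time to fill progress before interacting; movement or release cancels it.
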(event Custom|UpdateByTimer
  (CallFunction|DetectInteractablesinRange (Variables|Trace|GetDraw%20Debug) (Variables|Trace|GetTimeForUpdate))
  (CallFunction|UpdateInteractable))

(event Custom|InteractBegin
  (bind _interactableref (Variables|Ref|GetInteractableRef))
  (Utilities|IsValid _interactableref
    (:Is%20Valid
      (bind _type (Class|BPIInteractable|GetInteractionType(Message) _interactableref))
      (switch Utilities|FlowControl|Switch|SwitchonE_InteractionType _type ; Check the type selected on object
        (:NewEnumerator0
          (CallFunction|InteractwithActive) ; Interact instantly if the Type is "Press"
        )
        (:NewEnumerator1
          (EventDispatchers|BindEventtoOnGoingInteractStart (EventDispatchers|CreateEvent :!event Custom|OnInteractionOnGoing)))))))

(event Custom|OnInteractionOnGoing
  (params (ElapsedSeconds :type Float%20%28double-precision%29))
  ;[0.15 0.15 0.15 0.5] When enum type is "Hold", bind an event and check if the elapsed time since pressed is greater than the wanted value
  (bind _duration (Class|BPIInteractable|GetHoldDuration(Message) (Variables|Ref|GetInteractableRef)))
  (bind _interactionwidget (Variables|Ref|GetInteractionWidget)
    (:then
      (Default|SetProgressPercent _interactionwidget (/ ElapsedSeconds _duration)))
    (:else
      _))
  (if (> ElapsedSeconds _duration)
    (CallFunction|InteractwithActive)
    (EventDispatchers|UnbindEventfromOnGoingInteractStart (delegate Custom|OnInteractionOnGoing))))

(event Custom|InteractWithActive
  ;[0.15 0.15 0.15 0.5] Final interaction logic (called only when pressed or hold completed
  (Class|BPIInteractable|Interact(Message) (Variables|Ref|GetInteractableRef) (Variables|Ref|GetCharacterRef)))

(event Input|EnhancedActionEvents|EnhancedInputActionIA_Interact
  (params (ActionValue :type Boolean) (ElapsedSeconds :type Float%20%28double-precision%29) (TriggeredSeconds :type Float%20%28double-precision%29) (InputAction :type Input%20Action%20Object%20Reference :default "/Game/Input/Actions/IA_Interact.IA_Interact"))
  ;[0.15 0.15 0.15 0.5] Interaction input Handler
  (:Started
    (CallFunction|InteractBegin) ; Press event call
  )
  (:Ongoing
    (Default|CallOnGoingInteractStart ElapsedSeconds) ; Hold event dipatcher to avoid conflict
  )
  (:Canceled
    (CallFunction|CancelInteraction :!label _label))
  (:Completed
    (goto _label)))

(event Input|EnhancedActionEvents|EnhancedInputActionIA_Move
  (params (ActionValue :type Vector%202D%20Structure) (ElapsedSeconds :type Float%20%28double-precision%29) (TriggeredSeconds :type Float%20%28double-precision%29) (InputAction :type Input%20Action%20Object%20Reference :default "/Game/Input/Actions/IA_Move.IA_Move"))
  (:Started
    (CallFunction|CancelInteraction)))

(event EventBeginPlay
  (bind _ascharacter (Utilities|Casting|CastToCharacter (Components|GetOwner)))
  (Utilities|IsValid _ascharacter
    (:Is%20Valid
      (Variables|Ref|SetCharacterRef _ascharacter)
      (bind _returnvalue (Game|AddComponentbyClass (Components|GetOwner) "/Script/UMG.WidgetComponent" true))
      (Class|WidgetComponent|SetWidgetSpace _returnvalue "Screen")
      (Class|WidgetComponent|SetDrawSize _returnvalue "(X=100.000000,Y=100.000000)")
      (Variables|Ref|SetInteractionWidgetComponent _returnvalue)
      (Utilities|Time|SetTimerbyEvent (EventDispatchers|CreateEvent :!event Custom|UpdateByTimer) (Variables|Trace|GetTimeForUpdate) true))))

(fn UpdateInteractable
  (bind _activeinteractable (CallFunction|GetActiveInteractable))
  (if (and (Utilities|IsValid _activeinteractable) (!= _activeinteractable (Variables|Ref|GetInteractableRef)))
    (Variables|Ref|SetInteractableRef _activeinteractable)
    (elif (and (!= _activeinteractable (Variables|Ref|GetInteractableRef)) (not (Utilities|IsValid _activeinteractable)))
      (Variables|Ref|SetInteractableRef 0))))

(fn GetActiveInteractable
  (for (_array_element _array_index) (Variables|Ref|GetInteractablesInRange) ; Iterate over the actors in range
    (LocalVariables|SetCurrentActor _array_element)
    (if (== _array_index 0)
      ;[0.15 0.15 0.15 0.5] If it is the first actor in array set it to closest
      (LocalVariables|SetClosestActor (LocalVariables|GetCurrentActor))
      (else
        ;[0.15 0.15 0.15 0.5] Else find the closest to Character
        (LocalVariables|SetClosestActor (CallFunction|GetClosestActor (LocalVariables|GetCurrentActor) (LocalVariables|GetClosestActor))))))
  (return (LocalVariables|GetClosestActor)) ; End of the loop
)

(fn DitanceBeetwenActors
  (params (First :type Actor%20Object%20Reference) (Second :type Actor%20Object%20Reference))
  (return (Math|Vector|Distance(Vector) (Transformation|GetActorLocation First) (Transformation|GetActorLocation Second))))

(fn GetClosestActor
  (params (Current :type Actor%20Object%20Reference) (Other :type Actor%20Object%20Reference))
  (bind _characterref (Variables|Ref|GetCharacterRef))
  (if (< (CallFunction|DitanceBeetwenActors Current _characterref) (CallFunction|DitanceBeetwenActors Other _characterref))
    (return Current) ; Return Current
    (else
      (return Other) ; Return Other
    )))

(fn RenderInteractionWidget
  (bind _interactableref (Variables|Ref|GetInteractableRef))
  (bind _interactionwidgetcomponent (Variables|Ref|GetInteractionWidgetComponent))
  (Utilities|IsValid (Variables|Ref|GetInteractableRef)
    (:Is%20Valid
      (bind _type (Class|BPIInteractable|GetInteractionType(Message) (Variables|Ref|GetInteractableRef)))
      (bind _returnvalue (UserInterface|CreateWidget "/Game/UI/WB_InteractWidget.WB_InteractWidget_C" 0 _type))
      (bind _output_get (Variables|Ref|SetInteractionWidget _returnvalue))
      (UserInterface|SetWidget (Variables|Ref|GetInteractionWidgetComponent) _output_get)
      (bind _offsetcomp (Class|BPIInteractable|GetWidgetOffsetComp(Message) _interactableref))
      (Utilities|IsValid _offsetcomp
        (:Is%20Valid
          (Transformation|SetWorldLocation _interactionwidgetcomponent (Transformation|GetWorldLocation _offsetcomp) false false))
        (:Is%20Not%20Valid
          (Transformation|SetWorldLocation _interactionwidgetcomponent (Transformation|GetActorLocation _interactableref) false false))))
    (:Is%20Not%20Valid
      (UserInterface|SetWidget (Variables|Ref|GetInteractionWidgetComponent) 0))))

(fn CancelInteraction
  (bind _interactionwidget (Variables|Ref|GetInteractionWidget))
  (EventDispatchers|UnbindallEventsfromOnGoingInteractStart) ; Unbind all the events when the hold is completed or canceled
  (Utilities|IsValid _interactionwidget
    (:Is%20Valid
      (Default|SetProgressPercent _interactionwidget 0.0))))

(fn DetectInteractablesinRange
  (params (DrawDebug :type EDrawDebugTrace%20Enum :default "None") (DebugTime :type Float%20%28double-precision%29))
  (bind (_outactors _returnvalue) (Collision|SphereOverlapActors (Transformation|GetActorLocation (Variables|Ref|GetCharacterRef)) (Variables|Overlaps|GetRangeSphereRadius) (Variables|Trace|GetObject%20Types) 0))
  ;[0.15 0.15 0.15 0.5] For each overlapping actors, Check if it's an interactable AND can interact
  (for _array_element _outactors
    (bind _caninteract (Class|BPIInteractable|GetCanInteract(Message) _array_element))
    (if (Math|Boolean|ANDBoolean (Utilities|DoesObjectImplementInterface _array_element "/Game/Blueprint/Systems/InteractionSystem/BPI_Interactable.BPI_Interactable_C") _returnvalue _caninteract)
      (Utilities|Array|AddUnique (LocalVariables|GetActualInRange) _array_element)
      (bind (_outhit _returnvalue_2) (Collision|LineTraceForObjects (Transformation|GetActorLocation (Variables|Ref|GetCharacterRef)) (Transformation|GetActorLocation _array_element) (Variables|Trace|GetObject%20Types) false 0 DrawDebug true "(R=1.000000,G=0.000000,B=0.000000,A=1.000000)" "(R=0.000000,G=1.000000,B=0.000000,A=1.000000)" DebugTime))
      ;[0.15 0.15 0.15 0.5] If there is no obstacle between, add it to actual in range
      (if (not (and _returnvalue_2 (Utilities|DoesObjectImplementInterface (.HitActor (Collision|BreakHitResult _outhit)) "/Game/Blueprint/Systems/InteractionSystem/BPI_Interactable.BPI_Interactable_C")))
        (Utilities|Array|RemoveItem (LocalVariables|GetActualInRange) _array_element))))
  (CallFunction|SortActorsinRange (LocalVariables|GetActualInRange)))

(fn SortActorsinRange
  (params (AcutalInRange :type Array%20of%20Actor%20Object%20References))
  (bind _interactablesinrange (Variables|Ref|GetInteractablesInRange))
  (for _array_element AcutalInRange
    (if (== (Utilities|Array|FindItem _interactablesinrange _array_element) -1)
      (Utilities|Array|AddUnique (Variables|Ref|GetInteractablesInRange) _array_element)))
  (for _array_element_2 _interactablesinrange
    (if (== (Utilities|Array|FindItem AcutalInRange _array_element_2) -1)
      (Utilities|Array|AddUnique (LocalVariables|GetActorsToRemove) _array_element_2)))
  (for _array_element_3 (LocalVariables|GetActorsToRemove)
    (Utilities|Array|RemoveItem (Variables|Ref|GetInteractablesInRange) _array_element_3)))

(fn OnRepInteractableRef
  (CallFunction|RenderInteractionWidget))