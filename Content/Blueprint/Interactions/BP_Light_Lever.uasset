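; BP_Light_Lever is an interactable lever paired with a spotlight.
; Interact lights the spot, toggles the child-actor lever by message and broadcasts the interaction with itself as payload.
; TurnLightfor shows the light for a given time with an attenuated sound cue, using a timer to switch it off.
; Reset hides the light, returns the lever to inactive and disables interaction.
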(event Custom|TurnLightOff
  (Rendering|SetVisibility (Variables|Default|GetSpotLight) false false))

(event EventInteract
  (params (InteractActorRef :type Actor%20Object%20Reference))
  (Rendering|SetVisibility (Variables|Default|GetSpotLight) true false)
  (Class|BPILever|ToggleState(Message) (Variables|/Script/Engine.ChildActorComponent|GetChildActor (Variables|Default|GetBP_Lever_Clone)))
  (Default|CallCallInteraction self))

(event EventReset
  (Rendering|SetVisibility (Variables|Default|GetSpotLight) false false)
  (CallFunction|SetLeverState false)
  (Variables|Default|SetCan%20Interact false))

(event EventTurnLightfor
  (params (WaitFor :type Float%20%28double-precision%29) (TimeToLight :type Float%20%28double-precision%29))
  (Rendering|SetVisibility (Variables|Default|GetSpotLight) true false)
  (CallFunction|PlaySound "/Game/SoundAssets/Spotlight_Cue.Spotlight_Cue")
  (Utilities|Time|SetTimerbyEvent (delegate Custom|TurnLightOff) TimeToLight))

(fn ConstructionScript)

(fn SetCanInteract
  (params (canInteract :type Boolean))
  (Variables|Default|SetCan%20Interact canInteract))

(fn TurnLight
  (params (isOn :type Boolean))
  (Rendering|SetVisibility (Variables|Default|GetSpotLight) isOn false))

(fn SetLeverState
  (params (newIsActive :type Boolean))
  (Class|BPILever|SetState(Message) (Variables|/Script/Engine.ChildActorComponent|GetChildActor (Variables|Default|GetBP_Lever_Clone)) newIsActive))

(fn PlaySound
  (params (Sound :type Sound%20Base%20Object%20Reference))
  (Audio|PlaySoundatLocation Sound (Transformation|GetActorLocation) "0, 0, 0" 1.0 1.0 0.0 "/Game/SoundAssets/SA_SpotLight.SA_SpotLight" 0 0 0))

(fn GetCanInteract
  (return (Variables|Default|GetCan%20Interact)))

(fn GetHoldDuration
  (return 0.0))

(fn GetInteractionType
  (return "NewEnumerator0"))

(fn GetWidgetOffsetComp
  (return 0))