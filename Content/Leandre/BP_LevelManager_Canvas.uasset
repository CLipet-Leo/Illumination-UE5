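; BP_LevelManager_Canvas is a level manager that drives bars and torch lighting through the stages of a card-themed level.
; Two trigger volumes react to BP_ThirdPersonCharacter, toggle entrance or room bars, then destroy themselves; the room trigger also toggles the room and Red King torches.
; Custom events for King, Queen, Valet, Princess and level end toggle red and blue torches to advance the lighting.
; Toggles are relative, so results depend on initial states and call order.
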(event OnActorBeginOverlap(Trigger_StartLevel)
  (params (OverlappedActor :type Actor%20Object%20Reference) (OtherActor :type Actor%20Object%20Reference))
  (Utilities|Casting|CastToBP_ThirdPersonCharacter OtherActor)
  (Default|ToggleBars (Variables|Bars|GetEntranceBars))
  (Actor|DestroyActor (Variables|Triggers|GetTrigger_StartLevel)))

(event OnActorBeginOverlap(Trigger_Room)
  (params (OverlappedActor :type Actor%20Object%20Reference) (OtherActor :type Actor%20Object%20Reference))
  (Utilities|Casting|CastToBP_ThirdPersonCharacter OtherActor)
  (Default|ToggleBars (Variables|Bars|GetCardsBars))
  (Default|ToggleBars (Variables|Bars|GetObjectsBars))
  (Default|ToggleBars (Variables|Bars|GetRoomBars))
  (Actor|DestroyActor (Variables|Triggers|GetTrigger_Room))
  (Default|On/OffLight (Variables|Torches|GetTorch_Room))
  (Default|On/OffLight (Variables|Torches|GetTorch_Red_King)))

(event Custom|KingToQueen
  (Default|On/OffLight (Variables|Torches|GetTorch_Red_King))
  (Default|On/OffLight (Variables|Torches|GetTorch_Red_Queen))
  (Default|On/OffLight (Variables|Torches|GetTorch_Blue_King)))

(event Custom|QueenToValet
  (Default|On/OffLight (Variables|Torches|GetTorch_Red_Queen))
  (Default|On/OffLight (Variables|Torches|GetTorch_Red_Valet))
  (Default|On/OffLight (Variables|Torches|GetTorch_Blue_Queen)))

(event Custom|ValetToPrincess
  (Default|On/OffLight (Variables|Torches|GetTorch_Red_Valet))
  (Default|On/OffLight (Variables|Torches|GetTorch_Red_Princess))
  (Default|On/OffLight (Variables|Torches|GetTorch_Blue_Valet)))

(event Custom|EndOfLevel
  (Default|On/OffLight (Variables|Torches|GetTorch_Red_Princess))
  (Default|On/OffLight (Variables|Torches|GetTorch_Blue_Princess))
  (Default|On/OffLight (Variables|Torches|GetTorch_Room)))

(event EventBeginPlay)

(event Collision|EventActorBeginOverlap
  (params (OtherActor :type Actor%20Object%20Reference)))

(event EventTick
  (params (DeltaSeconds :type Float%20%28single-precision%29)))

(fn ConstructionScript)