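; BP_Lever_Clone is an interactable lever that toggles between two states, swinging Cube1 in pitch from its starting rotation.
; ToggleState inverts Activated and SetState applies only changed values; both feed a FlipFlop that plays or reverses a Timeline and adds an audio component.
; The Timeline lerps pitch toward ActivatedOffset, zeroing roll and yaw.
; Interaction getters return fixed or empty values, so GetIsActive always reports false.
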(event EventBeginPlay
  (Variables|Default|SetBaseRotation (Variables|/Script/Engine.SceneComponent|GetRelativeRotation (Variables|Default|GetCube1))))

(event EventToggleState
  (bind _baserotation (Variables|Default|GetBaseRotation))
  (bind _pitch (Math|Rotator|BreakRotator _baserotation))
  (Development|PrintString "Hello")
  (Variables|Default|SetbActivated (not (Variables|Default|GetbActivated)))
  (Utilities|FlowControl|FlipFlop
    (:A
      (AddComponent|AddAudioComponent false)
      (bind _levertrack (Timeline|Timeline Play)
        (:Update
          (Transformation|SetRelativeRotation (Variables|Default|GetCube1) (Math|Rotator|MakeRotator 0.0 (Math|Float|Lerp _pitch (+ _pitch (.Pitch (Math|Rotator|BreakRotator (Variables|Default|GetActivatedOffset)))) _levertrack) 0.0) false false))))
    (:B
      (AddComponent|AddAudioComponent false)
      (Timeline|Timeline Reverse))))

(event EventSetState
  (params (newIsActive :type Boolean))
  (bind _baserotation (Variables|Default|GetBaseRotation))
  (bind _pitch (Math|Rotator|BreakRotator _baserotation))
  (if (!= newIsActive (Variables|Default|GetbActivated))
    (Variables|Default|SetbActivated newIsActive)
    (Utilities|FlowControl|FlipFlop
      (:A
        (AddComponent|AddAudioComponent false)
        (bind _levertrack (Timeline|Timeline Play)
          (:Update
            (Transformation|SetRelativeRotation (Variables|Default|GetCube1) (Math|Rotator|MakeRotator 0.0 (Math|Float|Lerp _pitch (+ _pitch (.Pitch (Math|Rotator|BreakRotator (Variables|Default|GetActivatedOffset)))) _levertrack) 0.0) false false))))
      (:B
        (AddComponent|AddAudioComponent false)
        (Timeline|Timeline Reverse)))))

(fn ConstructionScript)

(fn GetWidgetOffsetComp
  (return 0))

(fn GetHoldDuration
  (return 0.0))

(fn GetInteractionType
  (return "NewEnumerator0"))

(fn GetIsActive
  (return false))