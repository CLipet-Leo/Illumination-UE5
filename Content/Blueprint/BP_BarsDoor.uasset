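; BP_BarsDoor is a barred door meant to open when every required lever is activated.
; A timeline lerps the bars mesh from its closed location by an opening offset, and CloseDoor reverses it.
; CheckCombination tests the activated levers against the required set, with ordered mode only a printed placeholder.
; As wired, AddLeverToArray's nested Contains check never reaches Add or CheckCombination, and removing a lever never calls CloseDoor.
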(event Custom|OpenDoor
  (Variables|Default|SetbIsOpen true)
  (bind _doortrack (Timeline|DoorTimeline Play)
    (:Update
      (Transformation|SetWorldLocation (Variables|Default|GetSM_Bars) (Math|Vector|Lerp(Vector) (Variables|Default|GetClosedLocation) (+ (Variables|Default|GetClosedLocation) (Variables|Default|GetOpeningOffset)) _doortrack) false false))))

(event Custom|CloseDoor
  (Variables|Default|SetbIsOpen false)
  (bind _doortrack (Timeline|DoorTimeline Reverse)
    (:Update
      (Transformation|SetWorldLocation (Variables|Default|GetSM_Bars) (Math|Vector|Lerp(Vector) (Variables|Default|GetClosedLocation) (+ (Variables|Default|GetClosedLocation) (Variables|Default|GetOpeningOffset)) _doortrack) false false))))

(event EventBeginPlay
  (Variables|Default|SetClosedLocation (Transformation|GetWorldLocation (Variables|Default|GetSM_Bars))))

(fn ConstructionScript)

(fn AddLevertoArray
  (params (LeverActor :type Actor%20Object%20Reference))
  (if (Utilities|Array|ContainsItem (Variables|Default|GetActivatedLevers) LeverActor)
    (if (Utilities|Array|ContainsItem (Variables|Default|GetActivatedLevers) LeverActor)
      (return)
      (else
        (Utilities|Array|Add (Variables|Default|GetActivatedLevers) LeverActor)
        (CallFunction|CheckCombination)))
    (else
      (return))))

(fn CheckCombination
  (if (Variables|Default|GetbRequiresOrder)
    (Development|PrintString "I didn't do the Order Logic Yet")
    (else
      (LocalVariables|SetbIsLoopBroken true)
      (for _array_element (Variables|Default|GetRequiredLevers)
        (if (not (Utilities|Array|ContainsItem (Variables|Default|GetActivatedLevers) _array_element))
          (LocalVariables|SetbIsLoopBroken false)))
      (if (LocalVariables|GetbIsLoopBroken)
        (CallFunction|OpenDoor)))))

(fn RemoveLeverfromArray
  (params (LeverActor :type Actor%20Object%20Reference))
  (bind _returnvalue (Utilities|Array|RemoveItem (Variables|Default|GetActivatedLevers) LeverActor))
  (if _returnvalue
    (if (not (Variables|Default|GetbIsOpen))
      (return))
    (else
      (return))))