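; BP_Canvas is an interactable canvas actor that exposes what looks like a shared interaction interface, with no behavior of its own beyond toggling.
; ToggleState flips the IsInteractable flag, which GetIsActivated reports back.
; The other getters return a zero hold duration, a fixed interaction type and OffsetRoot as the widget offset component.
; BeginPlay and the construction script are empty.
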(event Custom|ToggleState
  (Variables|Default|SetbIsInteractable (not (Variables|Default|GetbIsInteractable))))

(event EventBeginPlay)

(fn ConstructionScript)

(fn GetHoldDuration
  (return 0.0))

(fn GetInteractionType
  (return "NewEnumerator0"))

(fn GetIsActivated
  (return (Variables|Default|GetbIsInteractable)))

(fn GetWidgetOffsetComp
  (return (Variables|Default|GetOffsetRoot)))